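; BP_KillZone is a trigger volume that respawns the player at a designated spawn object when they overlap it.
; On overlap with a PlayerCharacter, and only if SpawnObject is valid, it disables character movement.
; After a short delay it moves the player to the spawn object's location plus a height offset, then after another delay restores Walking movement.
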(event `self.ReceiveActorBeginOverlap`
  (params (OtherActor :type "Actor Object Reference"))
  (bind _spawnobject (`self.SpawnObject`))
  (bind _asplayer_character (cast `PlayerCharacter` OtherActor))
  (`/Engine/EditorBlueprintResources/StandardMacros.IsValid` _spawnobject
    (:`Is Valid`
      (bind _charactermovement (`Character.CharacterMovement` _asplayer_character))
      (`CharacterMovementComponent.DisableMovement` _charactermovement)
      (`KismetSystemLibrary.Delay` 1.0)
      (`self.K2_SetActorLocation` _asplayer_character (+ (`self.K2_GetActorLocation` _spawnobject) (`KismetMathLibrary.MakeVector` 0.0 0.0 (`self.HeightOffset`))) false false)
      (`KismetSystemLibrary.Delay` 1.0)
      (`CharacterMovementComponent.SetMovementMode` _charactermovement "MOVE_Walking" 0))))

(fn `UserConstructionScript`)