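; BP_RingManager is a manager Blueprint that respawns the rings of a ring game when they run low.
; On BeginPlay it records the transform of every BP_RingGameRing in the level.
; Its CheckRings event counts the current rings and, if fewer than two exist, waits briefly and then spawns a new ring at every saved transform.
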(event `self.ReceiveBeginPlay`
  (bind _outactors (`GameplayStatics.GetAllActorsOfClass` "/Game/Blueprints/BP_RingGameRing.BP_RingGameRing_C"))
  (for _array_element _outactors
    (`KismetArrayLibrary.Array_Add` (`self.RingTransforms`) (`self.GetTransform` _array_element))))

(event `CheckRings`
  (bind _outactors (`GameplayStatics.GetAllActorsOfClass` "/Game/Blueprints/BP_RingGameRing.BP_RingGameRing_C"))
  (if (< (`KismetArrayLibrary.Array_Length` _outactors) 2)
    (`KismetSystemLibrary.Delay` 1.0)
    (for _array_element (`self.RingTransforms`)
      (`|SpawnActorFromClass` "/Game/Blueprints/BP_RingGameRing.BP_RingGameRing_C" _array_element "Undefined" "OverrideRootScale" null null))))

(fn `UserConstructionScript`)