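; BP_HexagoneObject is a platform actor that periodically wobbles along the vertical axis and then returns, on its own random schedule.
; BeginPlay stores the initial location and, after a random delay, plays a wobble timeline that offsets the mesh's height from that origin.
; A short pause leads into a second timeline driven by a return curve, whose completion calls StartOver to repeat the cycle after another random wait.
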(event `self.ReceiveBeginPlay`
  (bind (_initialworldlocation_x _initialworldlocation_y _initialworldlocation_z) (`KismetMathLibrary.BreakVector` (`self.InitialWorldLocation`)))
  (bind (_initialworldlocation_x_2 _initialworldlocation_y_2 _initialworldlocation_z_2) (`KismetMathLibrary.BreakVector` (`self.InitialWorldLocation`)))
  (set `self.InitialWorldLocation` (`self.K2_GetActorLocation`))
  (`KismetSystemLibrary.Delay` (`KismetMathLibrary.RandomFloatInRange` 3.0 15.0))
  (bind (_direction _heightwobbletrack) (`Timeline|StartWobbleProcedure` :!via `PlayFromStart` :!label _label)
    (:`Update`
      (`SceneComponent.K2_SetWorldLocation` (`self.PlatformMesh`) (`KismetMathLibrary.MakeVector` _initialworldlocation_x_2 _initialworldlocation_y_2 (+ _heightwobbletrack _initialworldlocation_z_2)) false false))
    (:`Finished`
      (`KismetSystemLibrary.Delay` 0.5)
      (bind (_direction_2 _returncurve) (`Timeline|EndProcedure` :!via `PlayFromStart`)
        (:`Update`
          (`SceneComponent.K2_SetWorldLocation` (`self.PlatformMesh`) (`KismetMathLibrary.MakeVector` _initialworldlocation_x _initialworldlocation_y (+ _returncurve _initialworldlocation_z)) false false))
        (:`Finished`
          (`self.StartOver`))))))

(event `StartOver`
  (`KismetSystemLibrary.Delay` (`KismetMathLibrary.RandomFloatInRange` 5.0 17.0))
  (goto _label :!via `PlayFromStart`))

(fn `UserConstructionScript`)