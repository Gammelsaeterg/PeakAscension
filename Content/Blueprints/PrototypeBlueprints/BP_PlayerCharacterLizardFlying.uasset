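; Prototype player character for a flying lizard, moved by control-rotation-relative forward and side input with yaw and pitch look.
; Tick interpolates the mesh rotation toward the velocity direction, while a timeline started on BeginPlay rolls both wings to flap.
; BeginPlay also creates the pause menu and reminder widgets, pausing immediately if the game instance's GamePlayed flag is false.
; Pause and resume functions toggle game pause, input mode, cursor and menu.
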(event `InputAxis|SideDirection`
  (params (AxisValue :type "Float (single-precision)"))
  (`self.AddMovementInput` (* (`KismetMathLibrary.GetRightVector` (`self.GetControlRotation`)) (`self.SideBaseVelocity`)) AxisValue))

(event `InputAxis|ForwardDirection`
  (params (AxisValue :type "Float (single-precision)"))
  (`self.AddMovementInput` (`KismetMathLibrary.GetForwardVector` (`self.GetControlRotation`)) AxisValue))

(event `self.ReceiveBeginPlay`
  (`self.CheckForUI`)
  (`self.SpawnReminderUI`)
  (bind (_direction _wingroll) (`Timeline|FlapWings`)
    (:`Update`
      (`SceneComponent.K2_SetRelativeRotation` (`self.WingLeft`) (`KismetMathLibrary.MakeRotator` _wingroll) false false)
      (`SceneComponent.K2_SetRelativeRotation` (`self.WingRight`) (`KismetMathLibrary.MakeRotator` _wingroll 0.0 -180.0) false false))))

(event `InputAxis|TurnHorizontal`
  (params (AxisValue :type "Float (single-precision)"))
  (`self.AddControllerYawInput` AxisValue))

(event `InputAxis|TurnVertical`
  (params (AxisValue :type "Float (single-precision)"))
  (`self.AddControllerPitchInput` AxisValue))

(event `CheckForUI`
  ;[1 1 1] Pause items
  (bind _returnvalue (`|CreateWidget` "/Game/UI/Prototype/UI_Prototype.UI_Prototype_C" (`GameplayStatics.GetPlayerController` 0)))
  (set `self.CurrentPlayerPauseMenu` _returnvalue)
  (bind _asbp_default_game_instance (cast `/Game/Blueprints/BP_DefaultGameInstance` (`GameplayStatics.GetGameInstance`)))
  (if (not (`/Game/Blueprints/BP_DefaultGameInstance.bGamePlayed` _asbp_default_game_instance))
    (`self.PauseGame`)))

(event `InputAction|Jump`
  (params (Key :type "Key Structure"))
  (:`Pressed`
    (`self.Jump`)))

(event `InputAction|Pause`
  (params (Key :type "Key Structure"))
  ;[1 1 1] Pause items
  (:`Pressed`
    (`self.PauseGame`)))

(event `self.ReceiveTick`
  (params (DeltaSeconds :type "Float (single-precision)"))
  (`SceneComponent.K2_SetWorldRotation` (`self.Mesh`) (`KismetMathLibrary.RInterpTo` (`SceneComponent.K2_GetComponentRotation` (`self.Mesh`)) (`KismetMathLibrary.Conv_VectorToRotator` (`KismetMathLibrary.Normal` (`self.GetVelocity`))) DeltaSeconds 15.0) false false))

(fn `PauseGame`
  (`UserWidget.AddToViewport` (`self.CurrentPlayerPauseMenu`) 0)
  (`GameplayStatics.SetGamePaused` true)
  (`WidgetBlueprintLibrary.SetInputMode_UIOnlyEx` (`GameplayStatics.GetPlayerController` 0) (`self.CurrentPlayerPauseMenu`))
  (set `PlayerController.bShowMouseCursor` true (`GameplayStatics.GetPlayerController` 0)))

(fn `ResumeGame`
  (`GameplayStatics.SetGamePaused` false)
  (`WidgetBlueprintLibrary.SetInputMode_GameOnly` (`GameplayStatics.GetPlayerController` 0))
  (set `PlayerController.bShowMouseCursor` false (`GameplayStatics.GetPlayerController` 0))
  (`Widget.RemoveFromParent` (`self.CurrentPlayerPauseMenu`)))

(fn `SpawnReminderUI`
  (`/Engine/EditorBlueprintResources/StandardMacros.IsValid` (`self.ReminderUI`)
    (:`Is Not Valid`
      (bind _returnvalue (`|CreateWidget` "/Game/UI/Prototype/UI_PauseReminder.UI_PauseReminder_C" (`GameplayStatics.GetPlayerController` 0)))
      (bind _output_get (set `self.ReminderUI` _returnvalue))
      (`UserWidget.AddToViewport` _output_get 0))))

(fn `UserConstructionScript`)