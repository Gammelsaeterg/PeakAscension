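; BP_RingGameRing is a ring in a ring minigame that the player passes through, crediting the flying lizard character.
; EnableRing and DisableRing toggle the Ring component's query collision and visibility along with the Enabled flag.
; When a PlayerCharacter ends overlap, it calls CheckRings on every BP_RingManager before disabling itself.
; It then calls AddRing only if that character is a BP_PlayerCharacterLizardFlying.
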(event `EnableRing`
  (`PrimitiveComponent.SetCollisionEnabled` (`self.Ring`) "QueryOnly")
  (`SceneComponent.SetVisibility` (`self.Ring`) true false)
  (set `self.bEnabled` true))

(event `DisableRing`
  (set `self.bEnabled` false)
  (`PrimitiveComponent.SetCollisionEnabled` (`self.Ring`) "NoCollision")
  (`SceneComponent.SetVisibility` (`self.Ring`) false false))

(event `self.ReceiveActorEndOverlap`
  (params (OtherActor :type "Actor Object Reference"))
  (bind _asplayer_character (cast `PlayerCharacter` OtherActor))
  (bind _outactors (`GameplayStatics.GetAllActorsOfClass` "/Game/Blueprints/PrototypeBlueprints/BP_RingManager.BP_RingManager_C"))
  (for _array_element _outactors
    (`/Game/Blueprints/PrototypeBlueprints/BP_RingManager.CheckRings` _array_element))
  (`self.DisableRing`)
  (bind _asbp_player_character_lizard_flying (cast `/Game/Blueprints/PrototypeBlueprints/BP_PlayerCharacterLizardFlying` _asplayer_character))
  (`/Game/Blueprints/PrototypeBlueprints/BP_PlayerCharacterLizardFlying.AddRing` _asbp_player_character_lizard_flying))

(fn `UserConstructionScript`)