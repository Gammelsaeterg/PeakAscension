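; BP_HexaPlateObject is a hexagonal plate actor that repeatedly wobbles vertically and glows once StartPlate is called.
; BeginPlay caches its world location and puts a dynamic material instance on its meshes.
; A wobble timeline drives height offset, emissive color and strength; after a pause the glow clears and an end timeline applies a return curve.
; StartOver then replays the wobble after a random delay, staggering the cycles.
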(event `StartPlate`
  (bind (_initialworldlocation_x _initialworldlocation_y _initialworldlocation_z) (`KismetMathLibrary.BreakVector` (`self.InitialWorldLocation`)))
  (bind (_initialworldlocation_x_2 _initialworldlocation_y_2 _initialworldlocation_z_2) (`KismetMathLibrary.BreakVector` (`self.InitialWorldLocation`)))
  (bind _dynamicmaterial (`self.DynamicMaterial`))
  (bind _dynamicmaterial_2 (`self.DynamicMaterial`))
  (bind (_direction _heightwobbletrack _emissivestrength _colorchange) (`Timeline|NewWobbleProcedure` :!via `PlayFromStart` :!label _label)
    (:`Update`
      (`SceneComponent.K2_SetWorldLocation` (`self.PlatformMesh`) (`KismetMathLibrary.MakeVector` _initialworldlocation_x_2 _initialworldlocation_y_2 (+ _heightwobbletrack _initialworldlocation_z_2)) false false)
      (`MaterialInstanceDynamic.SetVectorParameterValue` _dynamicmaterial_2 "EmissiveColor" _colorchange)
      (`MaterialInstanceDynamic.SetScalarParameterValue` _dynamicmaterial_2 "EmissiveStrength" _emissivestrength))
    (:`Finished`
      (`KismetSystemLibrary.Delay` 0.5)
      (`MaterialInstanceDynamic.SetVectorParameterValue` :`self` _dynamicmaterial :`ParameterName` "EmissiveColor")
      (`MaterialInstanceDynamic.SetScalarParameterValue` _dynamicmaterial "EmissiveStrength" 0.0)
      (bind (_direction_2 _returncurve) (`Timeline|EndProcedure` :!via `PlayFromStart`)
        (:`Update`
          (`SceneComponent.K2_SetWorldLocation` (`self.PlatformMesh`) (`KismetMathLibrary.MakeVector` _initialworldlocation_x _initialworldlocation_y (+ _returncurve _initialworldlocation_z)) false false))
        (:`Finished`
          (`self.StartOver`))))))

(event `self.ReceiveBeginPlay`
  (bind _returnvalue (`KismetMaterialLibrary.CreateDynamicMaterialInstance` (`PrimitiveComponent.GetMaterial` (`self.NewPlate`) 0)))
  (bind _output_get (set `self.DynamicMaterial` _returnvalue))
  (`PrimitiveComponent.SetMaterial` (`self.PlatformMesh`) 0 _output_get)
  (`PrimitiveComponent.SetMaterial` (`self.NewPlate`) 0 _output_get)
  (set `self.InitialWorldLocation` (`self.K2_GetActorLocation`)))

(event `StartOver`
  (`KismetSystemLibrary.Delay` (`KismetMathLibrary.RandomFloatInRange` 0.2 7.0))
  (goto _label :!via `PlayFromStart`))

(fn `UserConstructionScript`)