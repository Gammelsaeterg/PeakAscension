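; Moving ring actor for a ring game prototype that shuttles its Ring component back and forth along RingSpline.
; Each Tick runs the parent logic, then advances a normalized CurrentTime by MoveRate, with the Flipped flag setting the sign.
; A step that would leave the 0–1 range flips direction instead of moving.
; Ring is placed at the spline's world location using constant-velocity sampling, without sweep.
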(event `self.ReceiveTick`
  (params (DeltaSeconds :type "Float (single-precision)"))
  (`parent.ReceiveTick` DeltaSeconds)
  (`self.MoveRing` DeltaSeconds))

(event `FlipDirection`
  (if (`self.bFlipped`)
    (set `self.bFlipped` false)
    (else
      (set `self.bFlipped` true))))

(event `MoveRing`
  (params (DeltaSeconds :type "Float (double-precision)"))
  (bind _currenttime (`self.CurrentTime`))
  (bind _returnvalue (/ (* DeltaSeconds (`self.MoveRate`) (select `bool` (`self.bFlipped`) :`false` 1.0 :`true` -1.0 :!type "Float (single-precision)")) 100.0))
  (if (> (+ _returnvalue _currenttime) 1.0)
    (`self.FlipDirection`)
    (elif (< (+ _returnvalue (`self.CurrentTime`)) 0.0)
      (`self.FlipDirection`)
      (else
        (bind _output_get (set `self.CurrentTime` (+ _returnvalue _currenttime)))
        (`SceneComponent.K2_SetWorldLocation` (`self.Ring`) (`SplineComponent.GetLocationAtTime` (`self.RingSpline`) _output_get "World" true) false false)))))

(fn `UserConstructionScript`
  (`parent.UserConstructionScript`))