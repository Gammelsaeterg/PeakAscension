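; Prototype third-person player character with camera-relative movement, controller-driven look and a checkpoint respawn.
; Tick turns only the mesh toward velocity, holding the last remembered yaw when idle.
; Jump launches the grounded character up and slightly along the mesh's facing instead of using the standard Jump.
; BeginPlay saves the first checkpoint; pause and reminder UI functions exist, but their setup and calls here are disconnected.
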(event `RotatePlayerTowardsDirection`
  (params (DeltaTime :type "Float (double-precision)"))
  (bind _returnvalue (`self.GetVelocity`))
  (bind (_lastrememberedrotation_roll _lastrememberedrotation_pitch _lastrememberedrotation_yaw) (`KismetMathLibrary.BreakRotator` (`self.LastRememberedRotation`)))
  (bind _returnvalue_2 (`KismetMathLibrary.Conv_VectorToRotator` _returnvalue))
  (bind (_returnvalue_roll _returnvalue_pitch _returnvalue_yaw) (`KismetMathLibrary.BreakRotator` (`KismetMathLibrary.RInterpTo_Constant` (`SceneComponent.K2_GetComponentRotation` (`self.Mesh`)) _returnvalue_2 DeltaTime 720.0)))
  (if (> (`KismetMathLibrary.VSize` _returnvalue) 5.0)
    (set `self.LastRememberedRotation` _returnvalue_2)
    (`SceneComponent.K2_SetWorldRotation` (`self.Mesh`) (`KismetMathLibrary.MakeRotator` _returnvalue_roll _returnvalue_pitch _returnvalue_yaw) false false)
    (else
      (`SceneComponent.K2_SetWorldRotation` (`self.Mesh`) (`KismetMathLibrary.MakeRotator` 0.0 0.0 _lastrememberedrotation_yaw) false false))))

(event `ResetRotation`
  (bind (_lastrememberedrotation_roll _lastrememberedrotation_pitch _lastrememberedrotation_yaw) (`KismetMathLibrary.BreakRotator` (`self.LastRememberedRotation`)))
  (`SceneComponent.K2_SetWorldRotation` (`self.Mesh`) (`KismetMathLibrary.MakeRotator` 0.0 0.0 _lastrememberedrotation_yaw) false false))

(event `self.ReceiveTick`
  (params (DeltaSeconds :type "Float (single-precision)"))
  (set `self.CurrentDeltaTime` DeltaSeconds)
  (`self.RotatePlayerTowardsDirection` (`self.CurrentDeltaTime`)))

(event `SetCheckpoint`
  (bind (_returnvalue_location _returnvalue_rotation _returnvalue_scale) (`KismetMathLibrary.BreakTransform` (`self.GetTransform`)))
  (set `self.CurrentCheckpoint` (`KismetMathLibrary.MakeTransform` _returnvalue_location _returnvalue_rotation _returnvalue_scale))
  (`KismetSystemLibrary.PrintString` "CheckpointSet"))

(event `InputAxis|ForwardDirection`
  (params (AxisValue :type "Float (single-precision)"))
  (`self.AddMovementInput` (`KismetMathLibrary.GetForwardVector` (`KismetMathLibrary.MakeRotator` 0.0 0.0 (.yaw (`SceneComponent.K2_GetComponentRotation` (`self.Camera`))))) AxisValue))

(event `RespawnAtCheckpoint`
  (`self.K2_SetActorTransform` (`self.CurrentCheckpoint`))
  (`KismetSystemLibrary.PrintString` "Respawned")
  (`self.ResetRotation`))

(event `InputAxis|SideDirection`
  (params (AxisValue :type "Float (single-precision)"))
  (`self.AddMovementInput` (`KismetMathLibrary.GetRightVector` (`KismetMathLibrary.MakeRotator` 0.0 0.0 (.yaw (`SceneComponent.K2_GetComponentRotation` (`self.Camera`))))) AxisValue))

(event `InputAction|Jump`
  (params (Key :type "Key Structure"))
  (bind (_returnvalue_roll _returnvalue_pitch _returnvalue_yaw) (`KismetMathLibrary.BreakRotator` (`SceneComponent.K2_GetComponentRotation` (`self.Mesh`))))
  (bind _returnvalue (`KismetMathLibrary.MakeRotator` 0.0 0.0 _returnvalue_yaw))
  (:`Pressed`
    (if (not (`NavMovementComponent.IsFalling` (`self.CharacterMovement`)))
      (`self.LaunchCharacter` (* (`KismetMathLibrary.Normal` (+ (`KismetMathLibrary.GetForwardVector` _returnvalue) (* (`KismetMathLibrary.GetUpVector` _returnvalue) 4.0))) 600.0)))))

(event `InputAxis|TurnHorizontal`
  (params (AxisValue :type "Float (single-precision)"))
  (`self.AddControllerYawInput` AxisValue))

(event `InputAxis|TurnVertical`
  (params (AxisValue :type "Float (single-precision)"))
  (`self.AddControllerPitchInput` AxisValue))

(event `self.ReceiveBeginPlay`
  (`self.SetCheckpoint`))

(event `CheckForUI`
  ;[1 1 1] Pause items
)

(event `InputAction|Pause`
  (params (Key :type "Key Structure"))
  ;[1 1 1] Pause items
)

(fn `PauseGame`
  (`UserWidget.AddToViewport` (`self.CurrentPlayerPauseMenu`) 0)
  (`GameplayStatics.SetGamePaused` true)
  (`WidgetBlueprintLibrary.SetInputMode_UIOnlyEx` (`GameplayStatics.GetPlayerController` 0) (`self.CurrentPlayerPauseMenu`))
  (set `PlayerController.bShowMouseCursor` true (`GameplayStatics.GetPlayerController` 0)))

(fn `ResumeGame`
  (`GameplayStatics.SetGamePaused` false)
  (`WidgetBlueprintLibrary.SetInputMode_GameOnly` (`GameplayStatics.GetPlayerController` 0))
  (set `PlayerController.bShowMouseCursor` false (`GameplayStatics.GetPlayerController` 0))
  (`Widget.RemoveFromParent` (`self.CurrentPlayerPauseMenu`)))

(fn `SetPlayerIndexAndRot`
  (bind _output_get (set `self.PlayerIndex` 0))
  (`Controller.SetControlRotation` (`GameplayStatics.GetPlayerController` _output_get) (`KismetMathLibrary.MakeRotator` 0.0)))

(fn `SpawnReminderUI`
  (`/Engine/EditorBlueprintResources/StandardMacros.IsValid` (`self.ReminderUI`)
    (:`Is Not Valid`
      (bind _returnvalue (`|CreateWidget` "/Game/UI/Prototype/UI_PauseReminder.UI_PauseReminder_C" (`GameplayStatics.GetPlayerController` 0)))
      (bind _output_get (set `self.ReminderUI` _returnvalue))
      (`UserWidget.AddToViewport` _output_get 0))))

(fn `UserConstructionScript`)