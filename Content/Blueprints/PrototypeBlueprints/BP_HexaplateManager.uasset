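; BP_HexaplateManager is a prototype manager actor that triggers every hexaplate in the level one at a time in random order.
; On BeginPlay it gathers all BP_HexaPlateObject actors, shuffles them and waits a random few seconds.
; StartPlates then calls StartPlate on the current plate and re-invokes itself after another random delay until the last plate has started.
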(event `StartPlates`
  (`/Game/Blueprints/PrototypeBlueprints/BP_HexaPlateObject.StartPlate` (`|GetArrayItem` (`self.HexaplateArray`) (`self.CurrentIndex`)))
  (if (< (+ (`self.CurrentIndex`) 1) (`KismetArrayLibrary.Array_Length` (`self.HexaplateArray`)))
    (set `self.CurrentIndex` (+ (`self.CurrentIndex`) 1))
    (`KismetSystemLibrary.Delay` (`KismetMathLibrary.RandomFloatInRange` 3.0 7.0))
    (`self.StartPlates`)))

(event `self.ReceiveBeginPlay`
  (bind _outactors (`GameplayStatics.GetAllActorsOfClass` "/Game/Blueprints/PrototypeBlueprints/BP_HexaPlateObject.BP_HexaPlateObject_C"))
  (bind _output_get (set `self.HexaplateArray` _outactors))
  (`KismetArrayLibrary.Array_Shuffle` _output_get)
  (`KismetSystemLibrary.Delay` (`KismetMathLibrary.RandomFloatInRange` 3.0 7.0))
  (`self.StartPlates`))

(fn `UserConstructionScript`)