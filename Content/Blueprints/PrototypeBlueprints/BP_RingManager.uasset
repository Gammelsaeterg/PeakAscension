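; BP_RingManager is a manager for the ring game that re-enables the rings when they run low.
; It caches every BP_RingGameRing in the level on BeginPlay.
; CheckRings counts the enabled rings and, when fewer than two remain, waits briefly and calls EnableRing on all of them.
; Disconnected logic for saving ring transforms and respawning rings is left in the graph but never runs.
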(event `self.ReceiveBeginPlay`
  (bind _outactors (`GameplayStatics.GetAllActorsOfClass` "/Game/Blueprints/PrototypeBlueprints/BP_RingGameRing.BP_RingGameRing_C"))
  (set `self.RingActors` _outactors))

(event `CheckRings`
  (bind _enablecount (`self.EnableCount`))
  (set `self.EnableCount` 0)
  (for _array_element (`self.RingActors`)
    (if (`/Game/Blueprints/PrototypeBlueprints/BP_RingGameRing.bEnabled` _array_element)
      (set `self.EnableCount` (+ _enablecount 1))))
  (if (< _enablecount 2)
    (`KismetSystemLibrary.Delay` 2.0)
    (for _array_element_2 (`self.RingActors`)
      (`/Game/Blueprints/PrototypeBlueprints/BP_RingGameRing.EnableRing` _array_element_2))))

(fn `UserConstructionScript`)