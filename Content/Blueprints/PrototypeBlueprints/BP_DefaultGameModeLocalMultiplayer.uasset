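; Game mode for local multiplayer that creates the local players and their pawns when play begins.
; It caches all PlayerStarts, then for each index up to MaxPlayerCount finds those whose tag equals that index.
; At each match it creates the player, spawns and possesses a BP_PlayerDefault, sets its index and rotation, and records it in Players.
; InitializeSpawns reruns spawning, clearing the Players list without destroying existing pawns.
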(event `InitializeSpawns`
  (`self.SpawnPlayers`))

(event `self.ReceiveBeginPlay`
  (`self.GetPlayerStartPoints`)
  (`self.SpawnPlayers`))

(fn `GetPlayerStartPoints`
  (bind _outactors (`GameplayStatics.GetAllActorsOfClass` "/Script/Engine.PlayerStart"))
  (set `self.PlayerStartArray` _outactors))

(fn `SpawnPlayers`
  (bind _returnvalue (`GameplayStatics.GetPlayerController` (`self.Index`)))
  (if (> (`KismetArrayLibrary.Array_Length` (`self.Players`)) 0)
    (`KismetArrayLibrary.Array_Clear` (`self.Players`)))
  (for _index (range (`self.MaxPlayerCount`))
    (set `self.Index` _index)
    (for _array_element (`self.PlayerStartArray`)
      (if (`KismetStringLibrary.EqualEqual_StrStr` (`KismetStringLibrary.Conv_NameToString` (`PlayerStart.PlayerStartTag` _array_element)) (`KismetStringLibrary.Conv_IntToString` (`self.Index`)))
        (`GameplayStatics.CreatePlayer` (`self.Index`))
        (bind _returnvalue_2 (`|SpawnActorFromClass` "/Game/Blueprints/PrototypeBlueprints/BP_PlayerDefault.BP_PlayerDefault_C" (`self.GetTransform` _array_element) "AlwaysSpawn" "OverrideRootScale" null null))
        (`Controller.Possess` _returnvalue _returnvalue_2)
        (bind _asbp_player_default (cast `/Game/Blueprints/PrototypeBlueprints/BP_PlayerDefault` (`Controller.K2_GetPawn` _returnvalue)))
        (`/Game/Blueprints/PrototypeBlueprints/BP_PlayerDefault.SetPlayerIndexAndRot` _asbp_player_default)
        (`KismetArrayLibrary.Array_AddUnique` (`self.Players`) _returnvalue_2)))))

(fn `UserConstructionScript`)